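; SpeechRec is a Blueprint that lets the player open the Mrin_Gym level by voice command.
; On BeginPlay it binds StartGame to the speech recognition subsystem's words-spoken event.
; StartGame scans the recognized phrases for "Activate" and opens the level by name, with a boolean flag preventing repeat triggers.
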(event `self.ReceiveBeginPlay`
  (add `SpeechRecognitionSubsystem.OnWordsSpoken` (subsystem `SpeechRecognitionSubsystem`) (delegate `StartGame`)))

(event `StartGame`
  (params (Text :type "RecognisedPhrases Structure"))
  (for _array_element (`.phrases` (break `RecognisedPhrases` Text))
    (if (== _array_element "Activate")
      (if (not (`self.IsLevelActivated`))
        (`GameplayStatics.OpenLevel` "Mrin_Gym")
        (set `self.IsLevelActivated` true)))))

(fn `UserConstructionScript`)